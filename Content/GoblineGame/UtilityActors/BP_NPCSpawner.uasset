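; BP_NPCSpawner is a utility actor that spawns AI enemies at its own location, up to a maximum count.
; Each SpawnNPC call checks NPCCount against MaxNPCCount, spawns EnemyClassCharacter running BT_Enemy, sets the spawner as its owner and increments the count.
; Nothing in this graph triggers SpawnNPC or decrements the count.
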(event `self.SpawnNPC`
  (if (< (`self.NPCCount`) (`self.MaxNPCCount`))
    (bind _returnvalue (`AIBlueprintHelperLibrary.SpawnAIFromClass` (`self.EnemyClassCharacter`) "/Game/GoblineGame/Enemy/AI/BT_Enemy.BT_Enemy" (`self.K2_GetActorLocation`) (struct) false null))
    (`self.SetOwner` _returnvalue self)
    (set `self.NPCCount` (+ (`self.NPCCount`) 1))))

(fn `UserConstructionScript`)